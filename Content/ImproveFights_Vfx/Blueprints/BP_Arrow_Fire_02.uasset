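; Fire arrow projectile that flies via projectile movement at a configurable Speed and bursts on impact.
; BeginPlay passes the actor's up and right vectors to its projectile effect.
; On hit, it deactivates the effect, disables and hides the arrow, animates the effect's scale with a timeline, and spawns a half-size fire hit effect.
; Two delayed destroys follow, one after the timeline and one after the hit spawn; whichever fires first removes the actor.
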(event `self.ReceiveBeginPlay`
  (bind _effect_projectile (`self.Effect_Projectile`))
  (`FXSystemComponent.SetVectorParameter` _effect_projectile "User.UpVector" (`self.GetActorUpVector`))
  (`FXSystemComponent.SetVectorParameter` _effect_projectile "User.RightVector" (`self.GetActorRightVector`)))

(event `self.Arrow.OnComponentHit`
  (params (HitComponent :type "PrimitiveComponent Object Reference") (OtherActor :type "Actor Object Reference") (OtherComp :type "PrimitiveComponent Object Reference") (NormalImpulse :type "Vector Structure") (Hit :type "HitResult Structure (by ref)"))
  (bind _arrow (`self.Arrow`))
  (`|ExecutionSequence`
    (:`then_0`
      (`ActorComponent.Deactivate` (`self.Effect_Projectile`))
      (`PrimitiveComponent.SetSimulatePhysics` _arrow false)
      (`PrimitiveComponent.SetCollisionEnabled` _arrow "NoCollision")
      (`SceneComponent.SetVisibility` _arrow false false)
      (bind (_direction _newtrack_0) (`Timeline|Scale` :!via `PlayFromStart`)
        (:`Update`
          (`FXSystemComponent.SetFloatParameter` (`self.Effect_Projectile`) "User.Scale" _newtrack_0))
        (:`Finished`
          (`KismetSystemLibrary.Delay` 3.0)
          (`self.K2_DestroyActor`))))
    (:`then_1`
      (bind _returnvalue (`NiagaraFunctionLibrary.SpawnSystemAtLocation` "/Game/ImproveFights_Vfx/Particles/P_ArrowFire_Hit.P_ArrowFire_Hit" (`.ImpactPoint` (`GameplayStatics.BreakHitResult` Hit)) (`self.K2_GetActorRotation`)))
      (`FXSystemComponent.SetFloatParameter` _returnvalue "User.Size" 0.5)
      (`KismetSystemLibrary.Delay` 2.0)
      (`self.K2_DestroyActor`))))

(fn `UserConstructionScript`
  (set `ProjectileMovementComponent.InitialSpeed` (`self.Speed`) (`self.ProjectileMovement`)))