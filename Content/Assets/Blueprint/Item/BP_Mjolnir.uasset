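; Mjolnir weapon Blueprint that the third-person character equips in its hand socket, swings, drops and throws.
; While in use, a looping timer drives attacks, with socket box traces dealing damage; fast physics hits add damage and a sphere trace.
; Launch lerps it to an actor or point on a timeline, then reverses to the start position and reattaches.
; Timelines scale the Niagara aura that readies throws and fade the speed-triggered electricity trail.
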(event `self.ReceiveTick`
  (params (DeltaSeconds :type "Float (single-precision)"))
  (`self.TrailsWeapons`))

(event `/Game/Assets/Blueprint/Interface/BPI_Interaction.Use`
  (`self.PrevAttack`))

(event `/Game/Assets/Blueprint/Interface/BPI_Interaction.UnUse`
  (`self.StopAttack`))

(event `PrevAttack`
  ;[1 0.122 0.7312] Attack System
  (`KismetSystemLibrary.K2_ClearAndInvalidateTimerHandle` (`self.Event_Attack`))
  (bind _returnvalue (`KismetSystemLibrary.K2_SetTimerDelegate` (`|CreateDelegate` :!event `Attack`) 0.1 true))
  (set `self.Event_Attack` _returnvalue)
  (set `self.IsAttack` true))

(event `TrailsWeapons`
  (bind _p_electricity_trail (`self.P_Electricity_Trail`))
  (bind _p_electricity_trail_2 (`self.P_Electricity_Trail`))
  ;[0.4742 1 0.5065] Trails logic
  (if (and (`self.IsAttack`) (>= (`KismetMathLibrary.VSize` (`self.GetVelocity`)) 10.0))
    (if (not (`self.TrailWeapons`))
      (set `self.TrailWeapons` true)
      (`NiagaraComponent.ReinitializeSystem` _p_electricity_trail_2)
      (`ActorComponent.Activate` _p_electricity_trail_2 false)
      (`FXSystemComponent.SetFloatParameter` _p_electricity_trail_2 "User.StopParticles" 1.0)
      (`FXSystemComponent.SetFloatParameter` _p_electricity_trail_2 "User.Scale" 1.0))
    (elif (`self.TrailWeapons`)
      (set `self.TrailWeapons` false)
      (`NiagaraComponent.SetVariableFloat` _p_electricity_trail "User.StopParticles" 0.0)
      (bind (_direction _scale) (`Timeline|Deactivate_Trail` :!via `PlayFromStart`)
        (:`Update`
          (`NiagaraComponent.SetVariableFloat` _p_electricity_trail "User.Scale" _scale))
        (:`Finished`
          (`ActorComponent.Deactivate` _p_electricity_trail))))))

(event `Attack`
  (bind _ownertarget (`self.OwnerTarget`))
  (bind (_returnvalue_location _returnvalue_rotation) (`KismetMathLibrary.BreakTransform` (`SceneComponent.GetSocketTransform` (`self.StaticMesh`) "AttackSlot" "RTS_World")))
  ;[1 0.122 0.7312] Attack System
  (bind (_outhit _returnvalue) (`KismetSystemLibrary.BoxTraceSingle` _returnvalue_location _returnvalue_location (20.0 10.0 10.0) _returnvalue_rotation "TraceTypeQuery1" true (`|MakeArray` (`self.OwnerTarget`)) "ForOneFrame"))
  (if _returnvalue
    (bind (_bblockinghit _binitialoverlap _time _distance _location _impactpoint _normal _impactnormal _physmat _hitactor) (`GameplayStatics.BreakHitResult` _outhit))
    (`GameplayStatics.ApplyDamage` _hitactor 5.0 null (select `bool` (`KismetSystemLibrary.IsValid` _ownertarget) :`false` self :`true` _ownertarget :!type "Actor Object Reference"))
    (`NiagaraFunctionLibrary.SpawnSystemAtLocation` "/Game/ImproveFights_Vfx/Particles/P_Electricity_Hit.P_Electricity_Hit" _location)
    (`self.CheckThrowLogic` _hitactor)))

(event `StopAttack`
  ;[1 0.122 0.7312] Attack System
  (`KismetSystemLibrary.K2_ClearAndInvalidateTimerHandle` (`self.Event_Attack`))
  (set `self.IsAttack` false))

(event `/Game/Assets/Blueprint/Interface/BPI_Interaction.Equip`
  (params (Owner :type "Actor Object Reference"))
  ;[0.8184 0.3355 1] Pickup
  (bind _output_get (set `self.OwnerTarget` Owner))
  (`PrimitiveComponent.SetSimulatePhysics` (`self.StaticMesh`) false)
  (bind _asbp_third_person_character (cast `/Game/Assets/Blueprint/Player/BP_ThirdPersonCharacter` _output_get))
  (set `/Game/Assets/Blueprint/Player/BP_ThirdPersonCharacter.WeaponEquipped` true _asbp_third_person_character)
  (set `/Game/Assets/Blueprint/Player/BP_ThirdPersonCharacter.Weapons` self _asbp_third_person_character)
  (`self.K2_AttachToComponent` (`Character.Mesh` _asbp_third_person_character) "WeaponSocket" "SnapToTarget" "SnapToTarget" "KeepRelative"))

(event `/Game/Assets/Blueprint/Interface/BPI_Interaction.Drop`
  ;[0.08274 0.7685 1] Drop
  (bind _asbp_third_person_character (cast `/Game/Assets/Blueprint/Player/BP_ThirdPersonCharacter` (`self.OwnerTarget`))
    (:`then`
      (set `/Game/Assets/Blueprint/Player/BP_ThirdPersonCharacter.WeaponEquipped` false _asbp_third_person_character)
      (set `/Game/Assets/Blueprint/Player/BP_ThirdPersonCharacter.Weapons` null _asbp_third_person_character)
      (`self.K2_DetachFromActor` _asbp_third_person_character "KeepWorld" "KeepWorld" "KeepRelative"))
    (:`CastFailed`
      _))
  (set `self.OwnerTarget` null)
  (`PrimitiveComponent.SetSimulatePhysics` (`self.StaticMesh`) true))

(event `self.StaticMesh.OnComponentHit`
  (params (HitComponent :type "PrimitiveComponent Object Reference") (OtherActor :type "Actor Object Reference") (OtherComp :type "PrimitiveComponent Object Reference") (NormalImpulse :type "Vector Structure") (Hit :type "HitResult Structure (by ref)"))
  (bind _ownertarget (`self.OwnerTarget`))
  (bind _returnvalue (`SceneComponent.GetSocketLocation` (`self.StaticMesh`) "AttackSlot"))
  ;[1 0.3604 0.4302] Hit Component
  (if (>= (`KismetMathLibrary.VSize` (`self.GetVelocity`)) 350.0)
    (`GameplayStatics.ApplyDamage` OtherActor 5.0 null (`self.OwnerTarget`))
    (`self.CheckThrowLogic` OtherActor)
    (`NiagaraFunctionLibrary.SpawnSystemAtLocation` "/Game/ImproveFights_Vfx/Particles/P_Electricity_Hit.P_Electricity_Hit" (`.Location` (`GameplayStatics.BreakHitResult` Hit)))
    (bind (_outhit _returnvalue_2) (`KismetSystemLibrary.SphereTraceSingle` _returnvalue _returnvalue 60.0 "TraceTypeQuery1" false (`|MakeArray` (`self.OwnerTarget`))))
    (if _returnvalue_2
      (`GameplayStatics.ApplyDamage` (`.HitActor` (`GameplayStatics.BreakHitResult` _outhit)) 5.0 null (select `bool` (`KismetSystemLibrary.IsValid` _ownertarget) :`false` self :`true` _ownertarget :!type "Actor Object Reference")))))

(event `/Game/Assets/Blueprint/Interface/BPI_Interaction.CallAura`
  (params (Enabled :type Boolean))
  ;[0 1 0.8738] Aura Called
  (if Enabled
    (bind (_direction _scale) (`Timeline|AuraScale` :!via `Reverse` :!label _label)
      (:`Update`
        (`NiagaraComponent.SetVariableFloat` (`self.P_ElectricityAura`) "User.Scale" _scale))
      (:`Finished`
        (if Enabled
          (set `self.CanNowThrow` true))))
    (else
      (goto _label))))

(event `AuraCancelForced`
  ;[0 1 0.8738] Aura Called
  (`TimelineComponent.Stop` (`self.AuraScale`))
  (`NiagaraComponent.SetVariableFloat` (`self.P_ElectricityAura`) "User.Scale" 0.0))

(event `/Game/Assets/Blueprint/Interface/BPI_Interaction.CancelAura`
  ;[0 1 0.8738] Aura Called
  (set `self.CanNowThrow` false))

(event `/Game/Assets/Blueprint/Interface/BPI_Interaction.Launch`
  (params (ActorTarget :type "Actor Object Reference") (VectorTarget :type "Vector Structure"))
  ;[0.6332 1 0.06708] Launch Mjolnir
  (`/Engine/EditorBlueprintResources/StandardMacros.IsValid` ActorTarget
    (:`Is Valid`
      (set `self.TargetPos` (`self.K2_GetActorLocation` ActorTarget)))
    (:`Is Not Valid`
      (set `self.TargetPos` VectorTarget)))
  (`self.PrevAttack`)
  (set `self.LastPos` (`self.K2_GetActorLocation`))
  (set `self.IsThrow` true)
  (`self.CallAura` false)
  (bind _asbp_third_person_character (cast `/Game/Assets/Blueprint/Player/BP_ThirdPersonCharacter` (`self.OwnerTarget`)))
  (`self.K2_DetachFromActor` _asbp_third_person_character "KeepWorld" "KeepWorld" "KeepRelative")
  (`PrimitiveComponent.SetSimulatePhysics` (`self.StaticMesh`) true)
  (bind (_direction _move) (`Timeline|MoveToActor` :!label _label_2)
    (:`Update`
      (`self.K2_SetActorLocation` (`KismetMathLibrary.VLerp` (`self.LastPos`) (`self.TargetPos`) _move)))
    (:`Finished`
      (if (not (`self.IsHitTarget`))
        (set `self.IsHitTarget` true)
        (`self.ReverseTarget`)
        (set `self.IsThrow` false)
        (else
          (set `self.IsHitTarget` false)
          (`PrimitiveComponent.SetSimulatePhysics` (`self.StaticMesh`) false)
          (`self.StopAttack`)
          (bind _asbp_third_person_character_2 (cast `/Game/Assets/Blueprint/Player/BP_ThirdPersonCharacter` (`self.OwnerTarget`)))
          (`self.K2_AttachToComponent` (`Character.Mesh` _asbp_third_person_character_2) "WeaponSocket" "SnapToTarget" "SnapToTarget" "KeepRelative")
          (set `self.CanNowThrow` false))))))

(event `ReverseTarget`
  ;[0.6332 1 0.06708] Launch Mjolnir
  (goto _label_2 :!via `Reverse`))

(event `self.ReceiveBeginPlay`
  ;[0.6332 1 0.06708] Launch Mjolnir
  (`TimelineComponent.SetPlayRate` (`self.MoveToActor`) 3.0)
  (`TimelineComponent.SetPlayRate` (`self.AuraScale`) 0.3)
  (`self.CallAura` false))

(fn `CheckThrowLogic`
  (params (ActorTarget :type "Actor Object Reference"))
  (if (`self.IsThrow`)
    (message `/Game/Assets/Blueprint/Interface/BPI_EnemyLogic.DetectNearbyFriendly` ActorTarget)))

(fn `UserConstructionScript`)