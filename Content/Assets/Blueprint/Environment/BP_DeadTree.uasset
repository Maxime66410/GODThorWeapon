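; Dead tree prop that catches fire when DetectNearbyFriendly fires, burns down and shatters.
; Ignition happens once, spawning a fire emitter and a looping timer that drains Health while raising the dynamic material's Alpha.
; At zero Health it stops the fire, adds a geometry collection, triggers a short-lived FS_MasterField to break it and destroys the original Tree component.
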(event `self.ReceiveBeginPlay`
  (bind _returnvalue (`PrimitiveComponent.CreateDynamicMaterialInstance` (`self.Tree`) 0 (`PrimitiveComponent.GetMaterial` (`self.Tree`) 0) "None"))
  (set `self.InstancedMaterial` _returnvalue))

(event `/Game/Assets/Blueprint/Interface/BPI_EnemyLogic.DetectNearbyFriendly`
  (if (not (`self.IsFire`))
    (set `self.IsFire` true)
    (bind _returnvalue (`KismetSystemLibrary.K2_SetTimerDelegate` (`|CreateDelegate` :!event `RemoveHealth`) 0.1 true))
    (set `self.Event_Fire` _returnvalue)
    (bind _returnvalue_2 (`GameplayStatics.SpawnEmitterAtLocation` "/Game/Assets/Effects/M5VFXVOL2/Particles/Fire/Fire_08.Fire_08" (`SceneComponent.K2_GetComponentLocation` (`self.Tree`))))
    (set `self.FireEffect` _returnvalue_2)))

(event `RemoveHealth`
  (bind _instancedmaterial (`self.InstancedMaterial`))
  (`/Engine/EditorBlueprintResources/StandardMacros.DecrementFloat` (`self.Health`)
    (:`  `
      (bind _returnvalue (`MaterialInstanceDynamic.K2_GetScalarParameterValue` _instancedmaterial "Alpha"))
      (`MaterialInstanceDynamic.SetScalarParameterValue` _instancedmaterial "Alpha" (+ _returnvalue 0.01))
      (if (<= (`self.Health`) 0.0)
        (set `self.IsDeath` true)
        (`KismetSystemLibrary.K2_ClearAndInvalidateTimerHandle` (`self.Event_Fire`))
        (`ActorComponent.Deactivate` (`self.FireEffect`))
        (`AddComponent|NODE_AddGeometryCollectionComponent-0` :`RelativeTransform` (`KismetMathLibrary.MakeTransform` (0.0 0.0 0.0) (`self.K2_GetActorRotation`)))
        (bind _returnvalue_2 (`|SpawnActorFromClass` "/Engine/EditorResources/FieldNodes/FS_MasterField.FS_MasterField_C" (`KismetMathLibrary.MakeTransform` (`SceneComponent.K2_GetComponentLocation` (`self.Tree`)) (struct) (0.8 0.8 0.8)) "AlwaysSpawn" "MultiplyWithRoot" null null))
        (`/Engine/EditorResources/FieldNodes/FS_MasterField.CE_Trigger` _returnvalue_2)
        (`self.SetLifeSpan` _returnvalue_2 1.0)
        (`ActorComponent.K2_DestroyComponent` (`self.Tree`))))))

(fn `UserConstructionScript`)