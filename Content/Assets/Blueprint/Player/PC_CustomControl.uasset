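; Player controller that handles pickup and interaction input for the possessed third-person character.
; BeginPlay adds the default Enhanced Input mapping context, and possession caches the character reference.
; Pickup drops an equipped weapon, otherwise traces from the head socket along the follow camera's forward vector and sends an equip message to the hit actor.
; Interact runs the same trace and sends use and push messages to whatever it hits.
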(event `self.ReceiveBeginPlay`
  (bind _returnvalue (subsystem `EnhancedInputLocalPlayerSubsystem`))
  ;[0.04688 0.04688 0.04688] Init
  (`/Engine/EditorBlueprintResources/StandardMacros.IsValid` _returnvalue
    (:`Is Valid`
      (`EnhancedInputSubsystemInterface.AddMappingContext` _returnvalue "/Game/ThirdPerson/Input/IMC_Default.IMC_Default" 0 (struct)))))

(event `self.ReceivePossess`
  (params (PossessedPawn :type "Pawn Object Reference"))
  ;[0.1823 0.06234 0.02571] On Possess
  (bind _asbp_third_person_character (cast `/Game/Assets/Blueprint/Player/BP_ThirdPersonCharacter` PossessedPawn))
  (set `self.As BP Third Person Character` _asbp_third_person_character))

(event `EnhancedInput|/Game/Assets/Blueprint/Input/IA_Pickup`
  (params (ActionValue :type Boolean) (ElapsedSeconds :type "Float (double-precision)") (TriggeredSeconds :type "Float (double-precision)") (InputAction :type "InputAction Object Reference" :default "/Game/Assets/Blueprint/Input/IA_Pickup.IA_Pickup"))
  ;[1 0.6197 0.2776] Pickup items
  (:`Started`
    (bind _as_bp_third_person_character (`self.As BP Third Person Character`)
      (:`then`
        (if (`/Game/Assets/Blueprint/Player/BP_ThirdPersonCharacter.WeaponEquipped` _as_bp_third_person_character)
          (message `/Game/Assets/Blueprint/Interface/BPI_Interaction.Drop` (`/Game/Assets/Blueprint/Player/BP_ThirdPersonCharacter.Weapons` _as_bp_third_person_character))
          (else
            (bind _returnvalue (`SceneComponent.GetSocketLocation` (`Character.Mesh` _as_bp_third_person_character) "head"))
            (bind (_outhit _returnvalue_2) (`KismetSystemLibrary.LineTraceSingle` _returnvalue (+ _returnvalue (* (`KismetMathLibrary.GetForwardVector` (`SceneComponent.K2_GetComponentRotation` (`/Game/Assets/Blueprint/Player/BP_ThirdPersonCharacter.FollowCamera` _as_bp_third_person_character))) 500)) "TraceTypeQuery1" false (`|MakeArray` _as_bp_third_person_character :!type "Actor Object Reference")))
            (if _returnvalue_2
              (message `/Game/Assets/Blueprint/Interface/BPI_Interaction.Equip` (`.HitActor` (`GameplayStatics.BreakHitResult` _outhit)) (`self.As BP Third Person Character`))))))
      (:`else`))))

(event `EnhancedInput|/Game/Assets/Blueprint/Input/IA_Interact`
  (params (ActionValue :type Boolean) (ElapsedSeconds :type "Float (double-precision)") (TriggeredSeconds :type "Float (double-precision)") (InputAction :type "InputAction Object Reference" :default "/Game/Assets/Blueprint/Input/IA_Interact.IA_Interact"))
  ;[0.942 0.1428 1] Interact
  (:`Started`
    (bind _as_bp_third_person_character (`self.As BP Third Person Character`)
      (:`then`
        (bind _returnvalue (`SceneComponent.GetSocketLocation` (`Character.Mesh` _as_bp_third_person_character) "head"))
        (bind (_outhit _returnvalue_2) (`KismetSystemLibrary.LineTraceSingle` _returnvalue (+ _returnvalue (* (`KismetMathLibrary.GetForwardVector` (`SceneComponent.K2_GetComponentRotation` (`/Game/Assets/Blueprint/Player/BP_ThirdPersonCharacter.FollowCamera` _as_bp_third_person_character))) 500)) "TraceTypeQuery1" false (`|MakeArray` _as_bp_third_person_character :!type "Actor Object Reference")))
        (if _returnvalue_2
          (bind (_bblockinghit _binitialoverlap _time _distance _location _impactpoint _normal _impactnormal _physmat _hitactor) (`GameplayStatics.BreakHitResult` _outhit))
          (message `/Game/Assets/Blueprint/Interface/BPI_Interaction.Use` _hitactor)
          (message `/Game/Assets/Blueprint/Interface/BPI_Interaction.Push` _hitactor)))
      (:`else`))))

(fn `UserConstructionScript`)